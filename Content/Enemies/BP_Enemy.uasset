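; Enemy pawn Blueprint that roams the level and chases players who come near it.
; Roam loops AI MoveTo calls to random navigable points around its current location, repicking on success or failure.
; A proximity trigger overlap with a Player-tagged actor starts Chase, and ending that overlap returns to Roam.
; Chase moves to that actor, prints the outcome and resumes roaming; a debug-location spawn is left unconnected.
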(event `self.ReceiveBeginPlay`
  (`self.Roam`))

(event `Roam`
  (bind _randomlocation (`NavigationSystemV1.K2_GetRandomLocationInNavigableRadius` (`self.K2_GetActorLocation`) 2000.0 null null))
  (`|AIMoveTo` self _randomlocation null
    (:`OnSuccess`
      _)
    (:`OnFail`
      _))
  (`self.Roam`))

(event `self.Proximity_Trigger.OnComponentBeginOverlap`
  (params (OverlappedComponent :type "PrimitiveComponent Object Reference") (OtherActor :type "Actor Object Reference") (OtherComp :type "PrimitiveComponent Object Reference") (OtherBodyIndex :type Integer) (bFromSweep :type Boolean) (SweepResult :type "HitResult Structure (by ref)"))
  (if (`self.ActorHasTag` OtherActor "Player")
    (`self.Chase` OtherActor)))

(event `self.Proximity_Trigger.OnComponentEndOverlap`
  (params (OverlappedComponent :type "PrimitiveComponent Object Reference") (OtherActor :type "Actor Object Reference") (OtherComp :type "PrimitiveComponent Object Reference") (OtherBodyIndex :type Integer))
  (if (`self.ActorHasTag` OtherActor "Player")
    (`self.Roam`)))

(event `Chase`
  (params (PlayerToChase :type "Actor Object Reference"))
  (`|AIMoveTo` self (0.0 0.0 0.0) PlayerToChase
    (:`OnSuccess`
      (`KismetSystemLibrary.PrintString` "gottem!"))
    (:`OnFail`
      (`KismetSystemLibrary.PrintString` "ah dangit")))
  (`self.Roam`))

(fn `UserConstructionScript`)